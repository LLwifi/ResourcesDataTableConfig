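; Sound actor whose volume follows how directly the player camera looks at it.
; Overlap by an autonomous-proxy actor opens a Tick gate; ending overlap mutes the audio and closes it.
; While open, it optionally rotates toward the camera and lowers volume as the angle from camera forward grows, scaled by AngleScale and floored at zero.
; A debug print of the multiplier and angle runs every gated tick.
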(event `self.ReceiveBeginPlay`)

(event `self.ReceiveTick`
  (params (DeltaSeconds :type "Float (single-precision)"))
  (bind _returnvalue (`GameplayStatics.GetPlayerCameraManager` 0))
  (bind _returnvalue_2 (`self.K2_GetActorLocation`))
  (bind _returnvalue_3 (`PlayerCameraManager.GetCameraLocation` _returnvalue))
  (bind _returnvalue_4 (`KismetMathLibrary.DegAcos` (`KismetMathLibrary.Dot_VectorVector` (`KismetMathLibrary.Normal` (`KismetMathLibrary.Conv_RotatorToVector` (`PlayerCameraManager.GetCameraRotation` _returnvalue))) (`KismetMathLibrary.Normal` (- _returnvalue_2 _returnvalue_3)))))
  (bind _returnvalue_5 (- 1.0 (* (/ _returnvalue_4 180.0) (`self.AngleScale`))))
  (`/Engine/EditorBlueprintResources/StandardMacros.Gate` true :!label _label
    (:`Exit`
      (`|ExecutionSequence`
        (:`then_0`
          (if (`self.IsLookPlayer`)
            (`self.K2_SetActorRotation` (`KismetMathLibrary.FindLookAtRotation` _returnvalue_2 _returnvalue_3))))
        (:`then_1`
          (`AudioComponent.SetVolumeMultiplier` (`self.SoundAssetTagAudioComponent`) (select `bool` (> _returnvalue_5 0.0) :`true` _returnvalue_5))
          (`KismetSystemLibrary.PrintString` (`KismetStringLibrary.Concat_StrStr` (`KismetStringLibrary.Conv_DoubleToString` _returnvalue_5) "----默认角度" (`KismetStringLibrary.Conv_DoubleToString` _returnvalue_4)) true true (struct :`G` 0.66 :`B` 1.0 :`A` 1.0) 0.0))))))

(event `self.OnBeginOverlap`
  (params (OverlappedComponent :type "PrimitiveComponent Object Reference") (OtherActor :type "Actor Object Reference") (OtherComp :type "PrimitiveComponent Object Reference") (OtherBodyIndex :type Integer) (bFromSweep :type Boolean) (SweepResult :type "HitResult Structure (by ref)"))
  (`parent.OnBeginOverlap` OverlappedComponent OtherActor OtherComp OtherBodyIndex bFromSweep SweepResult)
  (if (`|EnumEquality` (`self.GetLocalRole` OtherActor) "ROLE_AutonomousProxy")
    (set `self.Player` OtherActor)
    (goto _label :!via `Open`)))

(event `self.OnEndOverlap`
  (params (OverlappedComponent :type "PrimitiveComponent Object Reference") (OtherActor :type "Actor Object Reference") (OtherComp :type "PrimitiveComponent Object Reference") (OtherBodyIndex :type Integer))
  (`parent.OnEndOverlap` OverlappedComponent OtherActor OtherComp OtherBodyIndex)
  (`AudioComponent.SetVolumeMultiplier` (`self.SoundAssetTagAudioComponent`) 0.0)
  (set `self.Player` null)
  (goto _label :!via `Close`))

(fn `UserConstructionScript`
  (`parent.UserConstructionScript`))